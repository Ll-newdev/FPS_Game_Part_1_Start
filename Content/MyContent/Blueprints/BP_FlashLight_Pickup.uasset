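; BP_FlashLight_Pickup is a world pickup that gives the first-person player a flashlight.
; On BeginPlay it caches the player character cast to BP_FirstPersonCharacter.
; When that character overlaps its collision component, it sets the character's HasFlashLight flag, plays a collect sound at its location and destroys itself.
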(event `self.ReceiveBeginPlay`
  ; set up
  (bind _asbp_first_person_character (cast `/Game/StarterContent/FirstPerson/Blueprints/BP_FirstPersonCharacter` (`GameplayStatics.GetPlayerCharacter` 0)))
  (set `self.Playerref` _asbp_first_person_character))

(event `self.Colllision.OnComponentBeginOverlap`
  (params (OverlappedComponent :type "PrimitiveComponent Object Reference") (OtherActor :type "Actor Object Reference") (OtherComp :type "PrimitiveComponent Object Reference") (OtherBodyIndex :type Integer) (bFromSweep :type Boolean) (SweepResult :type "HitResult Structure (by ref)"))
  (bind _playerref (`self.Playerref`))
  ; collect flashlight
  (if (== OtherActor _playerref)
    (set `/Game/StarterContent/FirstPerson/Blueprints/BP_FirstPersonCharacter.HasFlashLight` true _playerref)
    (`GameplayStatics.PlaySoundAtLocation` "/Game/MyContent/Audio/MP3_Key_Collect.MP3_Key_Collect" (`self.K2_GetActorLocation`) (struct) 1.0 1.0 0.0 null null null null)
    (`self.K2_DestroyActor`)))

(fn `UserConstructionScript`)