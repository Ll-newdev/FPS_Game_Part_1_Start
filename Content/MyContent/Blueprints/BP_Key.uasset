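; BP_Key is a key pickup that stays hidden and non-collidable until no BP_Target actors remain in the level.
; Each Tick it gathers the targets, using the index returned by an array Add as the count, and toggles visibility and collision.
; Player overlap then sets HasKey on BP_FirstPersonCharacter, plays a collect sound and destroys the key.
; The appear particle and sound effects are disconnected and never run.
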(event `self.ReceiveBeginPlay`
  ; setup
  (bind _asbp_first_person_character (cast `/Game/StarterContent/FirstPerson/Blueprints/BP_FirstPersonCharacter` (`GameplayStatics.GetPlayerCharacter` 0)))
  (set `self.PlayerRef` _asbp_first_person_character))

(event `self.ReceiveTick`
  (params (DeltaSeconds :type "Float (single-precision)"))
  ; functionalityof  key visibility
  (bind _outactors (`GameplayStatics.GetAllActorsOfClass` "/Game/MyContent/Blueprints/BP_Target.BP_Target_C"))
  (bind _returnvalue (`KismetArrayLibrary.Array_Add` _outactors))
  (bind _output_get (set `self.AllTargetsDestroyed` (<= _returnvalue 0)))
  (`SceneComponent.SetVisibility` (`self.SM_Key`) _output_get false)
  (`self.SetActorEnableCollision` _output_get))

(event `self.Collision.OnComponentBeginOverlap`
  (params (OverlappedComponent :type "PrimitiveComponent Object Reference") (OtherActor :type "Actor Object Reference") (OtherComp :type "PrimitiveComponent Object Reference") (OtherBodyIndex :type Integer) (bFromSweep :type Boolean) (SweepResult :type "HitResult Structure (by ref)"))
  ; collceting the key
  (if (and (== OtherActor (`self.PlayerRef`)) (`self.AllTargetsDestroyed`))
    (set `/Game/StarterContent/FirstPerson/Blueprints/BP_FirstPersonCharacter.HasKey` true (`self.PlayerRef`))
    (`GameplayStatics.PlaySoundAtLocation` "/Game/MyContent/Audio/MP3_Key_Collect.MP3_Key_Collect" (`self.K2_GetActorLocation`) (struct) 1.0 1.0 0.0 null null null null)
    (`self.K2_DestroyActor`)))

(fn `UserConstructionScript`)